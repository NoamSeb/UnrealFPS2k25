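; BP_Trap is a trap door that swings open when the level's BP_BigEyes actor signals it.
; On BeginPlay it finds that actor and binds to its EDOpenTrap dispatcher.
; When triggered, it plays a sound at its location through MSS_SFX, selected by an Index parameter.
; A timeline, with play rate scaled by AnimationTime, then rolls the Cube from 90 to 180 degrees.
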(event `self.ReceiveBeginPlay`
  (bind _returnvalue (`GameplayStatics.GetActorOfClass` "/Game/FirstPerson/Blueprints/BP_BigEyes.BP_BigEyes_C"))
  (add `/Game/FirstPerson/Blueprints/BP_BigEyes.ED_OpenTrap` _returnvalue (delegate `OpenTrapTrigger`)))

(event `OpenTrapTrigger`
  (bind _returnvalue (`GameplayStatics.SpawnSoundAtLocation` "/Game/FirstPerson/Sound/MetaSound/MSS_SFX.MSS_SFX" (`self.K2_GetActorLocation`) (struct) 1.0 1.0 0.0 null null))
  (`AudioParameterControllerInterface.SetIntParameter` _returnvalue "Index" 11)
  (`AudioComponent.Play` _returnvalue 0.0)
  (`self.OpenTrap`))

(event `OpenTrap`
  (`TimelineComponent.SetPlayRate` (`self.OpenTrapTimeline`) (/ 1.0 (`self.AnimationTime`)))
  (bind (_direction _dooropening) (`Timeline|OpenTrapTimeline` :!via `PlayFromStart`)
    (:`Update`
      (`SceneComponent.K2_SetRelativeRotation` (`self.Cube`) (`KismetMathLibrary.MakeRotator` (`KismetMathLibrary.Lerp` 90.0 180.0 _dooropening)) false false))))

(fn `UserConstructionScript`)